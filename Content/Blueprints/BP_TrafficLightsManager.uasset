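; BP_TrafficLightsManager runs a repeating timed color cycle on a traffic light.
; BeginPlay starts Recolor, a latent loop that steps through three enum-keyed states with a fixed Delay after each.
; Each step looks up its color in the ColorSettings map and passes it to ChangeColor, addressing only the first entry of the Light array.
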(event Custom|Recolor
  (bind _light (Variables|Default|GetLight))
  (bind _output (Utilities|Array|Get(acopy) _light))
  (bind _output_get (Variables|Default|SetColorSettings (Variables|Default|GetColorSettings) :!label _label))
  (Default|ChangeColor _output (.Value (Utilities|Map|Find (.colormap _output_get) "NewEnumerator0")))
  (Utilities|FlowControl|Delay 5.0)
  (Default|ChangeColor _output (.Value (Utilities|Map|Find (.colormap _output_get) "NewEnumerator1")))
  (Utilities|FlowControl|Delay 1.0)
  (Default|ChangeColor _output (.Value (Utilities|Map|Find (.colormap _output_get) "NewEnumerator2")))
  (Utilities|FlowControl|Delay 3.0)
  (goto _label))

(event EventBeginPlay
  (CallFunction|Recolor))

(event Collision|EventActorBeginOverlap
  (params (OtherActor :type Actor%20Object%20Reference)))

(event EventTick
  (params (DeltaSeconds :type Float%20%28single-precision%29)))

(fn ConstructionScript)